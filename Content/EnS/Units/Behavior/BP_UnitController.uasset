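; AI controller for EnS units that runs the unit behavior tree on the unit blackboard.
; Shortly after possessing an EnSUnit, it finds the unit's owning player character and writes an initial goal to the blackboard.
; That goal is a fixed distance from the unit along the owner mesh's right vector, with the vertical component of the offset flattened.
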(event `self.ReceiveBeginPlay`
  (bind _blackboardcomponent (`self.UseBlackboard` "/Game/EnS/Units/Behavior/BB_Unit.BB_Unit"))
  (`self.RunBehaviorTree` "/Game/EnS/Units/Behavior/BT_Unit.BT_Unit"))

(event `self.OnPossess`
  (params (PossessedPawn :type "Pawn Object Reference"))
  (`KismetSystemLibrary.Delay` 0.2)
  (bind _asen_sunit (cast `EnSUnit` PossessedPawn))
  (bind _ascharacter (cast `Character` (`EnSUnit.PlayerOwner` _asen_sunit)))
  (bind (_returnvalue_x _returnvalue_y) (`KismetMathLibrary.BreakVector` (* (`SceneComponent.GetRightVector` (`Character.Mesh` _ascharacter)) 1000.0)))
  (`BlackboardComponent.SetValueAsVector` (stale `self.ReceiveBeginPlay` _blackboardcomponent) (`self.GoalKey`) (+ (`KismetMathLibrary.MakeVector` _returnvalue_x _returnvalue_y 0.0) (`self.K2_GetActorLocation` _asen_sunit))))

(fn `UserConstructionScript`)