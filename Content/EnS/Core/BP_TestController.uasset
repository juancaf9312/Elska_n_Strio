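; Test player controller for mouse-driven, grid-based movement of a TopDownCharacter.
; Mouse axis input traces under the cursor and, when the hovered grid changes, runs grid pathfinding to feed a spawned PathGuide with hexagon decals.
; SetDestination moves the character to the clicked grid if within MoveRange.
; On arrival, it refreshes the visible movable grids, tracked with gameplay tags, keeping attackable grids visible when clearing.
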(event `self.ReceiveBeginPlay`
  (bind _pathguide (`self.PathGuide`))
  (bind _returnvalue (`|SpawnActorFromClass` "/Script/GridRuntime.PathGuide" (`KismetMathLibrary.MakeTransform` (0.0 0.0 0.0)) "AlwaysSpawn" "OverrideRootScale" null null))
  (set `self.PathGuide` _returnvalue)
  (`PathGuide.SetStartDecalMaterial` _pathguide "/Game/EnS/Materials/M_PathGuide_Hexagon.M_PathGuide_Hexagon")
  (`PathGuide.SetDestinationDecalMaterial` _pathguide "/Game/EnS/Materials/M_PathGuide_Hexagon.M_PathGuide_Hexagon"))

(event `InputAxis|Turn`
  (params (AxisValue :type "Float (single-precision)"))
  (bind (_bblockinghit _binitialoverlap _time _distance _location) (`GameplayStatics.BreakHitResult` (`self.GetHitResultUnderCursorForObjects` (`|MakeArray` "ObjectTypeQuery1" :!type "EObjectTypeQuery Enum"))))
  (if _bblockinghit :!label _label
    (bind _asbp_game_mode_test (cast `/Game/EnS/Core/BP_GameModeTest` (`GameplayStatics.GetGameMode`)))
    (bind _returnvalue (`GridManager.GetGridByPosition` (`/Game/EnS/Core/BP_GameModeTest.GridManager` _asbp_game_mode_test) _location))
    (if (!= _returnvalue (`self.CursorOverGrid`))
      (set `self.CursorOverGrid` _returnvalue)
      (`self.OnCursorOverGridChanged`))))

(event `InputAxis|LookUp`
  (params (AxisValue :type "Float (single-precision)"))
  (goto _label))

(event `InputAction|SetDestination`
  (params (Key :type "Key Structure"))
  (bind (_hitresult _returnvalue) (`self.GetHitResultUnderCursorForObjects` (`|MakeArray` "ObjectTypeQuery1" :!type "EObjectTypeQuery Enum")))
  (:`Pressed`
    (bind _astop_down_character (cast `/Game/EnS/Characters/TopDownCharacter` (`self.K2_GetPawn`)))
    (if _returnvalue
      (bind _returnvalue_2 (`GridPawnInterface.GetGridManager` _astop_down_character))
      ;[1 1 1] In Move Range
      (bind _returnvalue_3 (`GridManager.GetGridByPosition` _returnvalue_2 (`.Location` (`GameplayStatics.BreakHitResult` _hitresult))))
      (bind _returnvalue_4 (`GridManager.GetGridByPosition` _returnvalue_2 (`self.K2_GetActorLocation` _astop_down_character)))
      (bind _returnvalue_5 (`GridManager.GetDistance` _returnvalue_2 _returnvalue_4 _returnvalue_3))
      (if (<= _returnvalue_5 (`/Game/EnS/Characters/TopDownCharacter.MoveRange` _astop_down_character))
        (bind _succ (`/Game/EnS/Characters/TopDownCharacter.MoveTo` _astop_down_character _returnvalue_3))
        (`KismetSystemLibrary.PrintString` (`KismetStringLibrary.Conv_BoolToString` _succ))
        (if _succ
          (add `GridNavigationComponent.OnArrivalGoal` (`/Game/EnS/Characters/TopDownCharacter.GridNavigation` _astop_down_character) (delegate `ArrivalGoal`)))))))

(event `ArrivalGoal`
  (params (Component :type "GridNavigationComponent Object Reference"))
  (`self.UpdateMovableGrid` true))

(fn `ClearMovableGrid`
  (bind _movablegrids (`self.MovableGrids`))
  (for _array_element _movablegrids
    (bind _gridinfo (`Grid.GridInfo` _array_element))
    (bind _gameplaytags (`GridInfo.GameplayTags` _gridinfo))
    (`BlueprintGameplayTagLibrary.RemoveGameplayTag` _gameplaytags (struct :`TagName` "Grid.GridInfo.IsMovable"))
    (`GridInfo.Dirty` _gridinfo)
    (if (not (`BlueprintGameplayTagLibrary.HasTag` _gameplaytags (struct :`TagName` "Grid.GridInfo.IsAttackable")))
      (`Grid.SetVisibility` _array_element false)))
  (`KismetArrayLibrary.Array_Clear` _movablegrids))

(fn `OnCursorOverGridChanged`
  (bind _astop_down_character (cast `/Game/EnS/Characters/TopDownCharacter` (`self.K2_GetPawn`)))
  (bind _asbp_game_mode_test (cast `/Game/EnS/Core/BP_GameModeTest` (`GameplayStatics.GetGameMode`)))
  (bind _result (`GridManager.FindPath` (`/Game/EnS/Core/BP_GameModeTest.GridManager` _asbp_game_mode_test) (make `GridPathFindingRequest` _astop_down_character (`self.K2_GetActorLocation` _astop_down_character) (`Grid.GetCenter` (`self.CursorOverGrid`)))))
  (`PathGuide.SetPath` (`self.PathGuide`) _result))

(fn `UpdateMovableGrid`
  (params (NewVisibility :type Boolean))
  (`self.ClearMovableGrid`)
  (if NewVisibility
    (bind _astop_down_character (cast `/Game/EnS/Characters/TopDownCharacter` (`self.K2_GetPawn`)))
    (bind _returnvalue (`GridPawnInterface.GetGridManager` _astop_down_character))
    (bind _returnvalue_2 (`GridManager.GetGridByPosition` _returnvalue (`self.K2_GetActorLocation` _astop_down_character)))
    (bind _grids (`GridManager.GetGridsByRange` _returnvalue _returnvalue_2 (`/Game/EnS/Characters/TopDownCharacter.MoveRange` _astop_down_character)))
    (bind _output_get (set `self.MovableGrids` _grids))
    (for _array_element _output_get
      (`Grid.SetVisibility` _array_element true)
      (bind _gridinfo (`Grid.GridInfo` _array_element))
      (`BlueprintGameplayTagLibrary.AddGameplayTag` (`GridInfo.GameplayTags` _gridinfo) (struct :`TagName` "Grid.GridInfo.IsMovable"))
      (`GridInfo.Dirty` _gridinfo))))

(fn `UserConstructionScript`)