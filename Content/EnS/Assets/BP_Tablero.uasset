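; BP_Tablero is a board actor that lays out pillar instances through its BPPilar component, each with a height entry.
; The construction script adds one instance at the origin and one at each BPPilar socket, zeroing their heights and resizing HeightMap to match.
; Construction passes the zeroed Heights to BPPilar, while Tick overwrites them with HeightMap every frame and prints a debug string.
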(event `self.ReceiveBeginPlay`)

(event `self.ReceiveTick`
  (params (DeltaSeconds :type "Float (single-precision)"))
  (set `/Game/EnS/Assets/BP_Pilar.Heights` (`self.HeightMap`) (`self.BP_Pilar`))
  (`KismetSystemLibrary.PrintString` "Hello"))

(fn `AddSMInstance`
  (params (Transform :type "Transform Structure"))
  (`KismetArrayLibrary.Array_Add` (`self.Heights`))
  (`InstancedStaticMeshComponent.AddInstance` (`self.BP_Pilar`) Transform))

(fn `UserConstructionScript`
  (`KismetArrayLibrary.Array_Clear` (`self.Heights`))
  (`self.AddSMInstance` (`KismetMathLibrary.MakeTransform` (0.0 0.0 0.0)))
  (for _array_element (`SceneComponent.GetAllSocketNames` (`self.BP_Pilar`))
    (`self.AddSMInstance` (`SceneComponent.GetSocketTransform` (`self.BP_Pilar`) _array_element "RTS_Actor"))
    (`KismetArrayLibrary.Array_Resize` (`self.HeightMap`) (`KismetArrayLibrary.Array_Length` (`self.Heights`)))
    (set `/Game/EnS/Assets/BP_Pilar.Heights` (`self.Heights`) (`self.BP_Pilar`))))